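; Door actor that swings open and shut in response to its OpenDoor component's OnOpen and OnClose events, apparently driven by a pressure plate.
; The DoorSwing timeline plays or reverses, adding its OpenAngle yaw to the rotation cached at BeginPlay.
; A timeline event plays a lock or collapse sound, then flips IsClosed after a delay to prevent glitches and repeated sounds from quick retriggering.
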(event OnClose(OpenDoor)
  (bind _returnvalue (Transformation|GetActorLocation))
  ;[1 1 1] Prevents Glitching when activatng pressure plate in quick succession
  (if (not (Variables|Default|GetisClosed))
    (bind _open_angle (Timeline|Door%20Swing Reverse)
      (:Update
        (Transformation|SetActorRotation (Math|Rotator|CombineRotators (Math|Rotator|MakeRotator 0.0 0.0 _open_angle) (Variables|Default|GetInitial%20Rotation))))
      (:Sound%20Timing
        (if (Variables|Default|GetisClosed)
          (Audio|PlaySoundatLocation "/Game/Audio/door-lock.door-lock" _returnvalue)
          ;[1 1 1] stop sound playing when moving over plate
          (Utilities|FlowControl|Delay 1.5)
          (Variables|Default|SetisClosed false)
          (else
            (Audio|PlaySoundatLocation "/Game/StarterContent/Audio/Collapse01.Collapse01" _returnvalue)
            (Utilities|FlowControl|Delay 1.5)
            (Variables|Default|SetisClosed true)))))))

(event OnOpen(OpenDoor)
  (bind _returnvalue (Transformation|GetActorLocation))
  ;[1 1 1] Prevents Glitching when activatng pressure plate in quick succession
  (if (Variables|Default|GetisClosed)
    (bind _open_angle (Timeline|Door%20Swing Play)
      (:Update
        (Transformation|SetActorRotation (Math|Rotator|CombineRotators (Math|Rotator|MakeRotator 0.0 0.0 _open_angle) (Variables|Default|GetInitial%20Rotation))))
      (:Sound%20Timing
        (if (Variables|Default|GetisClosed)
          (Audio|PlaySoundatLocation "/Game/Audio/door-lock.door-lock" _returnvalue)
          ;[1 1 1] stop sound playing when moving over plate
          (Utilities|FlowControl|Delay 1.5)
          (Variables|Default|SetisClosed false)
          (else
            (Audio|PlaySoundatLocation "/Game/StarterContent/Audio/Collapse01.Collapse01" _returnvalue)
            (Utilities|FlowControl|Delay 1.5)
            (Variables|Default|SetisClosed true)))))))

(event EventBeginPlay
  (Variables|Default|SetInitial%20Rotation (Transformation|GetActorRotation))
  (Variables|Default|SetisClosed true))

(fn ConstructionScript)